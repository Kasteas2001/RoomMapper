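; BP_PaintZone is a paint surface actor that places and removes mesh instances on a plane, which the construction script sizes by Scale.
; AddInstance scales the relative location and snaps X and Y to a 100-unit grid; its proximity scan only breaks early, so the add still follows.
; RemoveInstance linearly searches the InstancedStaticMesh and deletes the first instance near the scaled location.
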(event Custom|AddInstance
  (params (NewRelativeLocation :type Vector))
  (bind _scale (Variables|Default|GetScale))
  (bind _instancedstaticmesh (Variables|Default|GetInstancedStaticMesh))
  (bind _returnvalue (* NewRelativeLocation _scale))
  (bind (_x _y) (Math|Vector|BreakVector _returnvalue))
  (bind _returnvalue_2 (Math|Float|%(Float) _y 1e+02))
  (bind _returnvalue_3 (Math|Float|%(Float) _x 1e+02))
  (bind _returnvalue_4 (- _y _returnvalue_2))
  (bind _returnvalue_5 (- _x _returnvalue_3))
  (bind _index (Utilities|FlowControl|ForLoopwithBreak 0 (- (Components|InstancedStaticMesh|GetInstanceCount _instancedstaticmesh) 1) :!label _label)
    (:LoopBody
      (if (Utilities|Operators|EqualEqual (* NewRelativeLocation (Variables|Default|GetScale)) (.Location (Math|Transform|BreakTransform (.OutInstanceTransform (Components|InstancedStaticMesh|GetInstanceTransform _instancedstaticmesh _index false)))) 51.0)
        (goto _label Break)))
    (:Completed
      (Components|InstancedStaticMesh|AddInstance _instancedstaticmesh (Math|Transform|MakeTransform (Math|Vector|MakeVector (Math|Float|SelectFloat (+ _returnvalue_5 1e+02) _returnvalue_5 (>= (Math|Float|%(Float) _returnvalue_3 5e+01) 1.0)) (Math|Float|SelectFloat (+ _returnvalue_4 1e+02) _returnvalue_4 (>= (Math|Float|%(Float) _returnvalue_2 5e+01) 1.0)) 0.0) "0, 0, 0" "1.000000,1.000000,1.000000") false))))

(event Custom|RemoveInstance
  (params (RelativeLocation :type Vector))
  (bind _instancedstaticmesh (Variables|Default|GetInstancedStaticMesh))
  (bind _returnvalue (Components|InstancedStaticMesh|GetInstanceCount _instancedstaticmesh))
  (bind _returnvalue_2 (- _returnvalue 1))
  (if (>= _returnvalue_2 0)
    (bind _index (Utilities|FlowControl|ForLoopwithBreak 0 _returnvalue_2 :!label _label)
      (:LoopBody
        (if (Utilities|Operators|EqualEqual (* RelativeLocation (Variables|Default|GetScale)) (.Location (Math|Transform|BreakTransform (.OutInstanceTransform (Components|InstancedStaticMesh|GetInstanceTransform _instancedstaticmesh _index false)))) 1e+02)
          (Class|InstancedStaticMeshComponent|RemoveInstance (Variables|Default|GetInstancedStaticMesh) _index)
          (goto _label Break))))))

(event EventBeginPlay)

(event Collision|EventActorBeginOverlap
  (params (OtherActor :type Actor%20Object%20Reference)))

(event EventTick
  (params (DeltaSeconds :type Float%20%28single-precision%29)))

(fn ConstructionScript
  (bind _scale (Variables|Default|GetScale))
  (Transformation|SetRelativeScale3D (Variables|Default|GetPlane) (Math|Vector|MakeVector _scale _scale 1.0)))